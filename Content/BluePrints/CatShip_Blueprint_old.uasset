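; Old cat ship Blueprint that continuously swivels its Child component in a periodic wobble.
; The construction script tilts the X and Y axes about Z by their cone angles.
; Tick advances a wrapped angle per axis by its period, spins those vectors around X and Y (X offset by InitialRotation), and sets Child's swept relative rotation from them.
; An earlier back-and-forth pitch animation and other rotation experiments remain disconnected.
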(event `self.ReceiveTick`
  (params (DeltaSeconds :type "Float (single-precision)"))
  (bind _returnvalue (* DeltaSeconds 360.0))
  ;[1 1 1] Progress The Swivel
  (set `self.Current Swivel X` (mod (+ (/ _returnvalue (`self.Swivel Period X`)) (`self.Current Swivel X`)) 360.0))
  (set `self.Current Swivel Y` (mod (+ (/ _returnvalue (`self.Swivel Period Y`)) (`self.Current Swivel Y`)) 360.0))
  (`SceneComponent.K2_SetRelativeRotation` (`self.Child`) (`KismetMathLibrary.MakeRotFromXY` (`KismetMathLibrary.RotateAngleAxis` (+ (`self.Swivel Axis X`) (`self.InitialRotation`)) (`self.Current Swivel X`) (1.0 0.0 0.0)) (`KismetMathLibrary.RotateAngleAxis` (`self.Swivel Axis Y`) (`self.Current Swivel Y`) (0.0 1.0 0.0))) true false))

(fn `UserConstructionScript`
  (set `self.Swivel Axis X` (`KismetMathLibrary.RotateAngleAxis` (1.0 0.0 0.0) (`self.Swivel Cone X`) (0.0 0.0 1.0)))
  (set `self.Swivel Axis Y` (`KismetMathLibrary.RotateAngleAxis` (0.0 1.0 0.0) (`self.Swivel Cone Y`) (0.0 0.0 1.0))))