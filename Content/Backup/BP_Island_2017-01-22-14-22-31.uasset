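; BP_Island is an actor whose cube the player pulls toward their pawn by looking at it and holding Fire.
; Each Tick, a component line trace along the camera's forward vector sets IsHovered, and Fire input sets MouseDown.
; When both flags are true, ApplyForce pushes the Cube horizontally along the direction to the pawn and prints the offset for debugging.
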(event `self.ReceiveBeginPlay`
  (bind _returnvalue (`GameplayStatics.GetPlayerController` 0))
  (`self.EnableInput` _returnvalue)
  (set `PlayerController.bEnableMouseOverEvents` true _returnvalue)
  (set `PlayerController.bEnableClickEvents` true _returnvalue))

(event `self.ReceiveTick`
  (params (DeltaSeconds :type "Float (single-precision)"))
  (bind _returnvalue (`GameplayStatics.GetPlayerCameraManager` 0))
  (bind _returnvalue_2 (`PlayerCameraManager.GetCameraLocation` _returnvalue))
  (bind _returnvalue_3 (- (`self.K2_GetActorLocation` (`GameplayStatics.GetPlayerPawn` 0)) (`SceneComponent.K2_GetComponentLocation` (`self.Cube`))))
  (bind (_returnvalue_x _returnvalue_y) (`KismetMathLibrary.BreakVector` (`KismetMathLibrary.Normal` _returnvalue_3)))
  (`|ExecutionSequence`
    (:`then_0`
      (if (`self.isHovered`)
        (if (`self.mouseDown`)
          (`KismetSystemLibrary.PrintString` (`KismetStringLibrary.Conv_VectorToString` _returnvalue_3))
          (`PrimitiveComponent.AddForce` (`self.Cube`) (* (`KismetMathLibrary.MakeVector` _returnvalue_x _returnvalue_y) 200000.0) "None" false))))
    (:`then_1`
      (bind (_hitlocation _hitnormal _bonename _returnvalue_4) (`PrimitiveComponent.K2_LineTraceComponent` (`self.Cube`) _returnvalue_2 (+ _returnvalue_2 (* (`KismetMathLibrary.GetForwardVector` (`PlayerCameraManager.GetCameraRotation` _returnvalue)) 1000000.0)) false false))
      (if _returnvalue_4
        (set `self.isHovered` true)
        (else
          (set `self.isHovered` false))))))

(event `InputAction|Fire`
  (params (Key :type "Key Structure" :default "AnyKey"))
  (:`Pressed`
    (set `self.mouseDown` true))
  (:`Released`
    (set `self.mouseDown` false)))

(fn `UserConstructionScript`)